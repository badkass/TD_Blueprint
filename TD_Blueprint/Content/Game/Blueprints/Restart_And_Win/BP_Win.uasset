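; BP_Win is a level-exit actor that advances the game when the player pawn overlaps it and no BP_Collectables actors remain in the level.
; It locates the current level in its LevelNames array and opens the next entry by name.
; On the last listed level, it instead prints a congratulations message and quits the game.
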(event `self.ReceiveActorBeginOverlap`
  (params (OtherActor :type "Actor Object Reference"))
  (if (== OtherActor (`GameplayStatics.GetPlayerPawn` 0))
    (if (not (`self.Any Collectable remaining`))
      (`self.Complete Level`))))

(fn `Any Collectable remaining`
  (returns (ReturnValue :type Boolean))
  (bind _outactors (`GameplayStatics.GetAllActorsOfClass` "/Game/Game/Blueprints/Collectables/BP_Collectables.BP_Collectables_C"))
  (return (> (`KismetArrayLibrary.Array_Length` _outactors) 0)))

(fn `Complete Level`
  (if (`self.Is Final level `)
    (`KismetSystemLibrary.PrintString` "Congratulations ! You collect all the items !")
    (`KismetSystemLibrary.QuitGame` null "Quit")
    (else
      (`self.Load Next Level`))))

(fn `Get Current Level Index`
  (returns (ReturnValue :type Integer))
  (bind _returnvalue (`GameplayStatics.GetCurrentLevelName` true))
  (return (`KismetArrayLibrary.Array_Find` (`self.Level Names`) (`KismetStringLibrary.Conv_StringToName` _returnvalue))))

(fn `Is Final level `
  (returns (`Return Value` :type Boolean))
  (return (== (`KismetArrayLibrary.Array_LastIndex` (`self.Level Names`)) (`self.Get Current Level Index`))))

(fn `Load Next Level`
  (`GameplayStatics.OpenLevel` (`|GetArrayItem` (`self.Level Names`) (+ (`self.Get Current Level Index`) 1))))

(fn `UserConstructionScript`)