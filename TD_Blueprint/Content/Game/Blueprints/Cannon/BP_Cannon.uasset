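; BP_Cannon is a cannon actor that fires BP_Projectile actors automatically and repeatedly from BeginPlay.
; Each cycle waits for CannonFirerate, then spawns a projectile at the spawn point's world location and rotation, scaled by ProjectileScale.
; A timeline then animates the barrel along its relative Y axis, and its Cannon Fired event track loops back to the delay for the next shot.
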(event `self.ReceiveBeginPlay`
  (`KismetSystemLibrary.Delay` (`self.Cannon_Firerate`) :!label _label)
  (`self.Spawn Projectiles`)
  (bind (_direction _cannon_barrell_location) (`Timeline|Cannon Fire Timeline` :!via `PlayFromStart`)
    (:`Update`
      (`self.Move Cannon Barell` _cannon_barrell_location))
    (:`Cannon Fired`
      (goto _label))))

(fn `Move Cannon Barell`
  (params (`Cannon Barell Y Location` :type "Float (double-precision)"))
  (`SceneComponent.K2_SetRelativeLocation` (`self.Cannon`) (`KismetMathLibrary.MakeVector` 0.0 `Cannon Barell Y Location`) false false))

(fn `Spawn Projectiles`
  (bind _projectils_spawn_point (`self.Projectils Spawn Point`))
  (`|SpawnActorFromClass` "/Game/Game/Blueprints/Cannon/BP_Projectile.BP_Projectile_C" (`KismetMathLibrary.MakeTransform` (`SceneComponent.K2_GetComponentLocation` _projectils_spawn_point) (`SceneComponent.K2_GetComponentRotation` _projectils_spawn_point) (`KismetMathLibrary.Conv_DoubleToVector` (`self.Projectile_Scale`))) "Undefined" "OverrideRootScale" null null))

(fn `UserConstructionScript`)